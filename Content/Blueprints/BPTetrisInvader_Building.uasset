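; Destructible building for a Tetris Invader game that absorbs bullets until its health runs out.
; Its Box overlap destroys each TetrisInvader_Bullet and decrements Health, then removes only the Box at zero so later bullets no longer register.
; Tick tints the Destructible's materials from green to red through a "Color" parameter, using Health relative to the value saved at BeginPlay.
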(event OnComponentBeginOverlap(Box)
  (params (OverlappedComponent :type Primitive%20Component%20Object%20Reference) (OtherActor :type Actor%20Object%20Reference) (OtherComp :type Primitive%20Component%20Object%20Reference) (OtherBodyIndex :type Integer) (bFromSweep :type Boolean) (SweepResult :type Hit%20Result%20Structure%20%28by%20ref%29))
  (bind _astetris_invader_bullet (Utilities|Casting|CastToTetrisInvader_Bullet OtherActor))
  (Actor|DestroyActor _astetris_invader_bullet)
  (if (> (Variables|Default|Gethealth) 0)
    (Variables|Default|Sethealth (- (Variables|Default|Gethealth) 1))
    (if (not (> (Variables|Default|Gethealth) 0))
      (Components|DestroyComponent (Variables|Default|GetBox)))))

(event EventBeginPlay
  (Variables|Default|SetInitHealth (Variables|Default|Gethealth)))

(event Collision|EventActorBeginOverlap
  (params (OtherActor :type Actor%20Object%20Reference)))

(event EventTick
  (params (DeltaSeconds :type Float%20%28single-precision%29))
  (Rendering|Material|SetVectorParameterValueonMaterials (Variables|Default|GetDestructible) "Color" (Math|Conversions|ToVector(LinearColor) (Math|Color|Lerp(LinearColor) "(R=1.000000,G=0.000000,B=0.000000,A=1.000000)" "(R=0.000000,G=1.000000,B=0.000000,A=1.000000)" (/ (Math|Conversions|ToFloat(Integer) (Variables|Default|Gethealth)) (Math|Conversions|ToFloat(Integer) (Variables|Default|GetInitHealth)))))))

(fn ConstructionScript)