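; BP_BreakoutBall is the physics-driven ball for a Breakout game, with events to launch and stop it, and it stores its start position.
; Every Tick rescales velocity to BallSpeed and snaps its heading to the nearest XY diagonal by rotating 45 degrees, rounding yaw to 90, and rotating back.
; Hits play block or paddle beeps, and the first hit on each of green, orange and red blocks raises BallSpeed.
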(event OnComponentHit(StaticMeshComponent)
  (params (HitComponent :type Primitive%20Component%20Object%20Reference) (OtherActor :type Actor%20Object%20Reference) (OtherComp :type Primitive%20Component%20Object%20Reference) (NormalImpulse :type Vector :default "0, 0, 0") (Hit :type Hit%20Result%20Structure%20%28by%20ref%29))
  ;[0.06505 0.4844 1] Ball Behaviour
  (Variables|Default|SethasTouchedPawn false)
  (Utilities|Casting|CastToBP_Block_Yellow OtherActor
    (:then
      (Audio|PlaySound2D "/Game/Sounds/457146__studiolittleman__8-bit-beeping-noise.457146__studiolittleman__8-bit-beeping-noise" 1.0 1.0 0.0 0 0 :!label _label))
    (:CastFailed
      (Utilities|Casting|CastToBP_Block_Green OtherActor
        (:then
          (if (Variables|Default|GethasTouchedGreen)
            (goto _label)
            (else
              (Variables|Default|SetBallSpeed (+ (Variables|Default|GetBallSpeed) 5e+01))
              (Variables|Default|SethasTouchedGreen true)
              (goto _label))))
        (:CastFailed
          (Utilities|Casting|CastToBP_Block_Orange OtherActor
            (:then
              (if (Variables|Default|GethasTouchedOrange)
                (goto _label)
                (else
                  (Variables|Default|SetBallSpeed (+ (Variables|Default|GetBallSpeed) 5e+01))
                  (Variables|Default|SethasTouchedOrange true)
                  (goto _label))))
            (:CastFailed
              (Utilities|Casting|CastToBP_Block_Red OtherActor
                (:then
                  (if (Variables|Default|GethasTouchedRed)
                    (goto _label)
                    (else
                      (Variables|Default|SetBallSpeed (+ (Variables|Default|GetBallSpeed) 5e+01))
                      (Variables|Default|SethasTouchedRed true)
                      (goto _label))))
                (:CastFailed
                  (Utilities|Casting|CastToBreakoutPawn OtherActor
                    (:then
                      (if (not (Variables|Default|GethasTouchedPawn))
                        (Variables|Default|SethasTouchedPawn true)
                        (Audio|PlaySound2D "/Game/Sounds/457146__studiolittleman__8-bit-beeping-noise2.457146__studiolittleman__8-bit-beeping-noise2" 1.0 1.0 0.0 0 0)))
                    (:CastFailed
                      (Utilities|Casting|CastToBP_Breakout_Pawn_Clone OtherActor)
                      (Audio|PlaySound2D "/Game/Sounds/457146__studiolittleman__8-bit-beeping-noise2.457146__studiolittleman__8-bit-beeping-noise2" 1.0 1.0 0.0 0 0))))))))))))

(event Custom|LaunchBall
  (Physics|AddImpulse (Variables|Debug|GetStaticMeshComponent) "1000.000000,-1000.000000, 0" "None" true))

(event Custom|VelocityAngleModifier
  (bind _returnvalue (Math|Rotator|MakeRotator 0.0 0.0 45.0))
  (bind _ballspeed (Variables|Default|GetBallSpeed))
  ;[0.2125 0.3106 1] MovementVelocity
  (bind _returnvalue_2 (Physics|GetPhysicsLinearVelocity (Variables|Debug|GetStaticMeshComponent) "None"))
  (Physics|SetPhysicsLinearVelocity (Variables|Debug|GetStaticMeshComponent) (* (Math|Vector|UnrotateVector (Math|Rotator|GetRotationXVector (Math|Rotator|MakeRotator 0.0 0.0 (Math|Conversions|ToFloat(Integer) (* (Math|Float|Round (/ (.yaw (Math|Rotator|MakeRotfromX (Math|Vector|RotateVector (Math|Vector|ClampVectorSize _returnvalue_2 _ballspeed _ballspeed) _returnvalue))) 9e+01)) 90)))) _returnvalue) (Math|Vector|VectorLength (Math|Vector|ClampVectorSize _returnvalue_2 _ballspeed _ballspeed))) false "None"))

(event Custom|StopBall
  (Physics|SetPhysicsLinearVelocity (Variables|Debug|GetStaticMeshComponent) "0, 0, 0" false "None"))

(event EventBeginPlay
  (Variables|Default|SetballStartPosition (Transformation|GetActorLocation)))

(event Collision|EventActorBeginOverlap
  (params (OtherActor :type Actor%20Object%20Reference)))

(event EventTick
  (params (DeltaSeconds :type Float%20%28single-precision%29))
  (CallFunction|VelocityAngleModifier))

(fn ConstructionScript)