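; Enemy controller for the Tetris Invader game that triggers a white-out transition once all enemies are dead.
; Tick watches the playing and all-enemies-died flags, then clears playing so the transition fires once.
; TransitionToWhite moves a target actor to a fixed X/Z at the player's Y, cubic-blends the view to it, then plays a FadeScreen widget's white fade-in.
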(event EventBeginPlay)

(event Collision|EventActorBeginOverlap
  (params (OtherActor :type Actor%20Object%20Reference)))

(event EventTick
  (params (DeltaSeconds :type Float%20%28single-precision%29))
  (if (and (Variables|Default|GetisPlaying) (Variables|Default|GetisAllEnemiesDied))
    (Variables|Default|SetisPlaying false)
    (Utilities|TransitiontoWhite 5.0 (Variables|Default|GetnewTarget))))

(fn ConstructionScript)