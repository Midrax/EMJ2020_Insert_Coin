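; Actor that runs the arcade-style continue screen, giving the player a timed chance to keep playing.
; BeginPlay creates the ContinueScreen widget, adds it to the viewport and plays its intro animation.
; Tick counts down CountdownTime, pushes the truncated seconds to the widget, and quits the game once time runs out.
; Pressing Fire calls Continue on MyGameInstance.
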(event EventBeginPlay
  (bind _returnvalue (UserInterface|CreateWidget "/Game/UI/ContinueScreen.ContinueScreen_C"))
  (bind _output_get (Variables|Default|SetcontinueScreenUI _returnvalue))
  (UserInterface|Viewport|AddtoViewport _output_get 0)
  (UserInterface|Animation|PlayAnimation _returnvalue (Variables|/Game/UI/ContinueScreen.ContinueScreen_C|GetAnimateIn (Variables|Default|GetcontinueScreenUI)) 0.0 1 "Forward" 1.0 false))

(event Collision|EventActorBeginOverlap
  (params (OtherActor :type Actor%20Object%20Reference)))

(event EventTick
  (params (DeltaSeconds :type Float%20%28single-precision%29))
  (if (> (Variables|Default|GetcountdownTime) 0.0)
    (bind _output_get (Variables|Default|SetcountdownTime (- (Variables|Default|GetcountdownTime) DeltaSeconds)))
    (Variables|/Game/UI/ContinueScreen.ContinueScreen_C|SetcountdownTime (Variables|Default|GetcontinueScreenUI) (Math|Float|Truncate _output_get))
    (else
      (Game|QuitGame 0 "Quit" false))))

(event Input|ActionEvents|InputActionFire
  (params (Key :type Key%20Structure :default "None"))
  (:Pressed
    (bind _asmy_game_instance (Utilities|Casting|CastToMyGameInstance (Game|GetGameInstance)))
    (Default|Continue _asmy_game_instance)))

(fn ConstructionScript)