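; Main menu controller that runs the title screen and the handoff into the Pong level.
; On BeginPlay it loops the MainMenu level sequence and shows the menu widget, chaining its animate-in into a looping animation.
; Fire, guarded to run once, sets game instance credits, swaps to the Intro sequence and animation, then uses timed delays for sounds and a Credits widget before opening Pong.
; F9 jumps straight to Breakout.
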(event EventBeginPlay
  (bind _outactor (Sequencer|Player|CreateLevelSequencePlayer "/Game/LevelSequence/MainMenu.MainMenu" (Utilities|Struct|MakeMovieSceneSequencePlaybackSettings true (Utilities|Struct|MakeMovieSceneSequenceLoopCount -1))))
  (Variables|Default|SetlevelSeqActor _outactor)
  (bind _returnvalue (UserInterface|CreateWidget "/Game/UI/MainMenuUI.MainMenuUI_C"))
  (bind _output_get (Variables|Default|SetMainMenuWidget _returnvalue))
  (UserInterface|Viewport|AddtoViewport _output_get 0)
  (Components|Animation|PlayAnimation _output_get (Variables|/Game/UI/MainMenuUI.MainMenuUI_C|GetAnimateIn _output_get) 0.0
    (:Finished
      (UserInterface|Animation|PlayAnimation _output_get (Variables|/Game/UI/MainMenuUI.MainMenuUI_C|GetLoop _output_get) 0.0 0 "Forward" 1.0 false))))

(event Collision|EventActorBeginOverlap
  (params (OtherActor :type Actor%20Object%20Reference)))

(event EventTick
  (params (DeltaSeconds :type Float%20%28single-precision%29)))

(event Input|ActionEvents|InputActionFire
  (params (Key :type Key%20Structure :default "None"))
  (bind _mainmenuwidget (Variables|Default|GetMainMenuWidget))
  (bind _mainmenuwidget_2 (Variables|Default|GetMainMenuWidget))
  (:Pressed
    (if (not (Variables|Default|GettransitioningToGame))
      (Variables|Default|SettransitioningToGame true)
      (bind _asmy_game_instance (Utilities|Casting|CastToMyGameInstance (Game|GetGameInstance)))
      (Variables|/Game/MyGameInstance.MyGameInstance_C|Setcredits _asmy_game_instance 10)
      (Class|UserWidget|StopAnimation _mainmenuwidget_2 (Variables|/Game/UI/MainMenuUI.MainMenuUI_C|GetLoop _mainmenuwidget_2))
      (Class|UserWidget|StopAnimationsandLatentActions _mainmenuwidget_2)
      (Actor|DestroyActor (Variables|Default|GetlevelSeqActor))
      (bind _outactor (Sequencer|Player|CreateLevelSequencePlayer "/Game/LevelSequence/Intro.Intro" (Utilities|Struct|MakeMovieSceneSequencePlaybackSettings true "(Value=0)" 1.0 0.0 false false false false false false false true)))
      (Variables|Default|SetlevelSeqActor _outactor)
      (UserInterface|Animation|PlayAnimation _mainmenuwidget (Variables|/Game/UI/MainMenuUI.MainMenuUI_C|GetIntro _mainmenuwidget) 0.0 1 "Forward" 1.0 false)
      (Audio|PlaySound2D "/Game/Sounds/213980__fenrirfangs__coin-clatter-2.213980__fenrirfangs__coin-clatter-2" 3.0 1.0 0.0 0 0)
      (Utilities|FlowControl|Delay 3.0)
      (bind _returnvalue (UserInterface|CreateWidget "/Game/UI/Credits.Credits_C"))
      (UserInterface|Viewport|AddtoViewport _returnvalue 0)
      (Audio|PlaySound2D "/Game/Sounds/182332__theonlypkmnmaster__8bit-vocal-synth.182332__theonlypkmnmaster__8bit-vocal-synth" 1.5 1.0 0.0 0 0)
      (Default|Init _mainmenuwidget)
      (Utilities|FlowControl|Delay 7.0)
      (Widget|RemovefromParent _mainmenuwidget)
      (Game|OpenLevel(byObjectReference) "/Game/Maps/Pong.Pong"))))

(event Input|KeyboardEvents|F9
  (params (Key :type Key%20Structure :default "None"))
  (:Pressed
    (Game|OpenLevel(byObjectReference) "/Game/Maps/Breakout.Breakout")))

(fn ConstructionScript)