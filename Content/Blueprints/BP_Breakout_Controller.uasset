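; Level controller for a Breakout stage that handles ball launch, out-of-bounds respawns costing a credit, score and the exit to the next level.
; It registers itself with every BP_Block, tracks remaining blocks and feeds the score widget each Tick.
; Once the ball has touched orange and the pawn, Tick eases blocks and top bound to new positions.
; At ten blocks left, it recenters the paddle, plays a sequence and opens TetrisInvader.
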(event EventBeginPlay
  ;[1 1 1] Block Controller Assignment
  (bind _outactors (Actor|GetAllActorsOfClass "/Game/Blueprints/BP_Block.BP_Block_C"))
  (Variables|Default|Setblocks _outactors)
  (for _array_element _outactors
    (Variables|/Game/Blueprints/BP_Block.BP_Block_C|Setcontroller _array_element self))
  (Variables|Default|SettotalBlocks (Utilities|Array|Length _outactors))
  (bind _returnvalue (UserInterface|CreateWidget "/Game/UI/BreakoutScore.BreakoutScore_C"))
  (Variables|Default|SetscoreUI _returnvalue)
  (UserInterface|Viewport|AddtoViewport _returnvalue 0))

(event Collision|EventActorBeginOverlap
  (params (OtherActor :type Actor%20Object%20Reference)))

(event EventTick
  (params (DeltaSeconds :type Float%20%28single-precision%29))
  (bind _breakoutball (Variables|Default|GetbreakoutBall))
  (bind _breakoutball_2 (Variables|Default|GetbreakoutBall))
  (bind _scoreui (Variables|Default|GetscoreUI))
  (bind _blockparent (Variables|Default|GetblockParent))
  (bind _topbound (Variables|Default|GettopBound))
  (bind _breakoutball_3 (Variables|Default|GetbreakoutBall))
  (bind _breakoutpawn (Variables|Default|GetbreakoutPawn))
  (bind _breakoutpawn_2 (Variables|Default|GetbreakoutPawn))
  (bind _returnvalue (Transformation|GetActorLocation _topbound))
  (bind _returnvalue_2 (Transformation|GetActorLocation _breakoutball_3))
  (bind _returnvalue_3 (Transformation|GetActorLocation _breakoutball_2))
  (bind _returnvalue_4 (Transformation|GetActorLocation _breakoutpawn))
  (bind _startposition (Variables|/Game/Characters/BreakoutPawn.BreakoutPawn_C|GetstartPosition _breakoutpawn))
  (Utilities|FlowControl|Sequence
    (:then_0
      ;[0.377 0.3496 1] LaunchBall
      (if (not (Variables|Default|GethasLaunched))
        (Transformation|SetActorLocation _breakoutball_2 (Math|Vector|MakeVector (.x _returnvalue_3) (.y (Transformation|GetActorLocation (Variables|Default|GetbreakoutPawn))) (.z _returnvalue_3)) false false)))
    (:then_1
      ;[1 1 1] RespawnPlayer
      (if (or (> (.x _returnvalue_2) 5.5e+02) (< (.x _returnvalue_2) -5.5e+02))
        (Variables|Default|SethasLaunched false)
        (Audio|PlaySound2D "/Game/Sounds/377338__samsterbirdies__space-gun-8-bit.377338__samsterbirdies__space-gun-8-bit" 0.4 1.0 0.0 0 0)
        (Transformation|SetActorLocation _breakoutpawn_2 (Variables|/Game/Characters/BreakoutPawn.BreakoutPawn_C|GetstartPosition _breakoutpawn_2) false false)
        (Transformation|SetActorLocation _breakoutball_3 (Variables|/Game/Blueprints/BP_BreakoutBall.BP_BreakoutBall_C|GetballStartPosition _breakoutball_3) false false)
        (Physics|SetPhysicsLinearVelocity (Variables|/Script/Engine.StaticMeshActor|GetStaticMeshComponent (Variables|Default|GetbreakoutBall)) "0, 0, 0" false "None")
        (bind _asmy_game_instance (Utilities|Casting|CastToMyGameInstance (Game|GetGameInstance)))
        (Default|ReduceCreditbyOne _asmy_game_instance)))
    (:then_2
      ;[0.3352 0.6074 1] Level Shift
      (if (and (Variables|/Game/Blueprints/BP_BreakoutBall.BP_BreakoutBall_C|GethasTouchedOrange _breakoutball) (Variables|/Game/Blueprints/BP_BreakoutBall.BP_BreakoutBall_C|GethasTouchedPawn _breakoutball))
        ;;[1 1 1] BlockParent
        (Transformation|SetActorLocation _blockparent (Math|Vector|MakeVector (Math|Interpolation|FInterpTo (.x (Transformation|GetActorLocation _blockparent)) -3.5e+02 DeltaSeconds 0.5) 0.0 0.0) false false)
        ;;[1 1 1] TopBound
        (Transformation|SetActorLocation _topbound (Math|Vector|MakeVector (.x _returnvalue) (Math|Interpolation|FInterpTo (.y _returnvalue) 1.7e+03 DeltaSeconds 0.5) (.z _returnvalue)) false false)
        ;;[1 1 1] Shift Sound
        (if (not (Variables|Default|GetisPlayingShiftEffect))
          (Audio|PlaySound2D "/Game/Sounds/breakoutshift.breakoutshift" 0.4 1.0 0.0 0 0)
          (Variables|Default|SetisPlayingShiftEffect true)
          (Default|PulseEffect (Variables|Default|GetpostProcess)))))
    (:then_3
      ;[0 0.06599 1] WinningTransition
      (if (Variables|Default|GetstartTransition)
        (Default|StopBall (Variables|Default|GetbreakoutBall))
        (Transformation|SetActorLocation _breakoutpawn (Math|Interpolation|VInterpTo _returnvalue_4 _startposition (Utilities|Time|GetWorldDeltaSeconds) 3.0) false false)
        (if (Math|Vector|Equal(Vector) _returnvalue_4 _startposition 0.1)
          (Variables|Default|SetstartTransition false)
          (Utilities|TransitiontoTetrisInvader))))
    (:then_4
      (Variables|/Game/UI/BreakoutScore.BreakoutScore_C|SetscoreToShow _scoreui (Variables|Default|Getscore))
      (Variables|/Game/UI/BreakoutScore.BreakoutScore_C|SetblocksLeft _scoreui (Variables|Default|GettotalBlocks)))))

(event Input|ActionEvents|InputActionFire
  (params (Key :type Key%20Structure :default "None"))
  ;[0.377 0.3496 1] LaunchBall
  (:Pressed
    (if (not (Variables|Default|GethasLaunched))
      (Default|LaunchBall (Variables|Default|GetbreakoutBall))
      (Variables|Default|SethasLaunched true)
      (Variables|/Game/UI/BreakoutScore.BreakoutScore_C|SetpromptVisibility (Variables|Default|GetscoreUI) "Hidden"))))

(fn ConstructionScript)

(fn DecrementBlock
  (if (> (Variables|Default|GettotalBlocks) 10)
    (bind _result (Math|Integer|DecrementInt (Variables|Default|GettotalBlocks))
      (:%20%20
        (Variables|Default|SettotalBlocks _result)))
    (else
      (Variables|Default|SetstartTransition true))))

(fn IncreaseScore
  (params (Amount :type Integer))
  (Variables|Default|Setscore (+ Amount (Variables|Default|Getscore))))

(fn DecrementBlock2
  (params (ActorToDelete :type Actor%20Object%20Reference))
  (bind _blocks (Variables|Default|Getblocks))
  (if (> (Utilities|Array|Length (Variables|Default|Getblocks)) 10)
    (if (Utilities|Array|ContainsItem _blocks ActorToDelete)
      (Utilities|Array|RemoveItem _blocks ActorToDelete))
    (else
      (Variables|Default|SetstartTransition true))))