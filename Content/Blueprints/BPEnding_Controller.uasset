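; BPEnding_Controller runs the game's ending sequence: an intro fade, the ending video, end credits, then a return to the main menu.
; On BeginPlay it adds the Ending widget, opens the video on the media player, and overlays a FadeScreen that fades out white.
; When the fade finishes, it removes that screen, rewinds, plays the UI intro animation and starts playback.
; The media end event hides the video, runs the credits animation, then opens MainMenu.
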(event Custom|OnVideoEnd
  (bind _ui (Variables|Default|GetUI))
  (Widget|SetVisibility (Variables|/Game/UI/Ending.Ending_C|GetVideo _ui) "Hidden")
  (|PlayAnimationTimeRange _ui (Variables|/Game/UI/Ending.Ending_C|GetRunEndCredit _ui) 0.0 0.0 1 "Forward" 1.0
    (:Finished
      (Game|OpenLevel(byObjectReference) "/Game/Maps/MainMenu.MainMenu"))))

(event EventBeginPlay
  (bind _mediaplayer (Variables|Default|GetMediaPlayer))
  (bind _mediaplayer_2 (Variables|Default|GetMediaPlayer))
  (bind _returnvalue (UserInterface|CreateWidget "/Game/UI/Ending.Ending_C"))
  (bind _output_get (Variables|Default|SetUI _returnvalue))
  (UserInterface|Viewport|AddtoViewport _output_get 0)
  (Media|MediaPlayer|OpenSource _mediaplayer "/Game/Movies/EMJ2020Ending.EMJ2020Ending")
  (Media|MediaPlayer|BindEventtoOnEndReached _mediaplayer (delegate Custom|OnVideoEnd))
  (bind _returnvalue_2 (UserInterface|CreateWidget "/Game/UI/FadeScreen.FadeScreen_C"))
  (UserInterface|Viewport|AddtoViewport _returnvalue_2 0)
  (Components|Animation|PlayAnimation _returnvalue_2 (Variables|/Game/UI/FadeScreen.FadeScreen_C|GetFadeOutWhite _returnvalue_2) 0.0
    (:Finished
      (Widget|RemovefromParent _returnvalue_2)
      (Class|MediaPlayer|Rewind _mediaplayer_2)
      (Utilities|FlowControl|Delay 0.1)
      (UserInterface|Animation|PlayAnimation (Variables|Default|GetUI) (Variables|/Game/UI/Ending.Ending_C|GetIn (Variables|Default|GetUI)) 0.0 1 "Forward" 1.0 false)
      (Media|MediaPlayer|Play _mediaplayer_2 :!class /Script/MediaAssets.MediaPlayer))))

(event Collision|EventActorBeginOverlap
  (params (OtherActor :type Actor%20Object%20Reference)))

(event EventTick
  (params (DeltaSeconds :type Float%20%28single-precision%29)))

(fn ConstructionScript)