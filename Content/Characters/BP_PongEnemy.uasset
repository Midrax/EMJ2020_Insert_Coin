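; BP_PongEnemy is the computer-controlled Pong paddle, a Cube that follows the ball along the Y axis.
; BeginPlay sets the tick interval from TickInterval, and each tick looks up BP_PongBall and caches its Sphere's relative location.
; Move then uses MoveComponentTo over TimeForMoving toward the ball's clamped Y.
; The relative move target takes its X, Z and rotation from the Cube's world transform.
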(event Custom|Move
  (bind _cube (Variables|Default|GetCube))
  (bind _returnvalue (Transformation|GetWorldTransform _cube))
  (Components|MoveComponentTo _cube (Math|Vector|MakeVector (.x (.location _returnvalue)) (Math|Float|Clamp(Float) (.y (Variables|Default|GetBall_Location)) -149.0 149.0) (.z (.location _returnvalue))) (.rotation _returnvalue) false false (Variables|Default|GetTimeForMoving) false))

(event EventBeginPlay
  (Actor|Tick|SetActorTickInterval (Variables|Default|GetTick%20Interval)))

(event Collision|EventActorBeginOverlap
  (params (OtherActor :type Actor%20Object%20Reference)))

(event EventTick
  (params (DeltaSeconds :type Float%20%28single-precision%29))
  (bind _returnvalue (Actor|GetActorOfClass "/Game/Characters/BP_PongBall.BP_PongBall_C"))
  (Variables|Default|SetBall_Location (Variables|/Script/Engine.SceneComponent|GetRelativeLocation (Variables|/Game/Characters/BP_PongBall.BP_PongBall_C|GetSphere _returnvalue)))
  (CallFunction|Move))

(fn ConstructionScript)